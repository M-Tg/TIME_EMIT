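; Laser enemy actor that casts a visible red beam forward from its root, drawn only as a debug line trace.
; Each Tick traces on Visibility, ending at the stored HitPosition if the previous trace hit, otherwise far ahead.
; Non-FirstPersonCharacter hits update HitPosition and print a debug "Hello"; character hits do nothing.
; A "Player" tag check exists but is never executed.
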(event `self.ReceiveTick`
  (params (DeltaSeconds :type "Float (single-precision)"))
  (bind _defaultsceneroot (`self.DefaultSceneRoot`))
  (bind _returnvalue (`SceneComponent.K2_GetComponentLocation` _defaultsceneroot))
  (bind _returnvalue_2 (`KismetMathLibrary.GetForwardVector` (`SceneComponent.K2_GetComponentRotation` _defaultsceneroot)))
  (if (`self.IsHit`)
    (set `self.endPosition` (`self.hitPosition`))
    (else
      (set `self.endPosition` (+ _returnvalue (* _returnvalue_2 10000.0)))))
  (bind (_outhit _returnvalue_3) (`KismetSystemLibrary.LineTraceSingle` :`Start` (+ (* _returnvalue_2 50.0) _returnvalue) :`End` (`self.endPosition`) :`TraceChannel` "TraceTypeQuery1" :`DrawDebugType` "ForOneFrame" :`TraceColor` (struct :`R` 1.0 :`B` 0.014804 :`A` 1.0) :`TraceHitColor` (struct :`R` 1.0) :`DrawTime` 1000.0))
  (bind _output_get (set `self.IsHit` _returnvalue_3))
  (if _output_get
    (bind (_bblockinghit _binitialoverlap _time _distance _location _impactpoint _normal _impactnormal _physmat _hitactor) (`GameplayStatics.BreakHitResult` _outhit))
    (cast `/Game/FirstPersonBP/Blueprints/FirstPersonCharacter` _hitactor
      (:`CastFailed`
        (set `self.hitPosition` _location)
        (`KismetSystemLibrary.PrintString` "Hello")))))

(fn `UserConstructionScript`)