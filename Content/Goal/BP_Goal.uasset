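; BP_Goal is a level goal with a sliding double door and an exit trigger.
; FirstPersonCharacter overlapping the actor starts opening it, and leaving the Sphere starts closing it.
; Tick ramps a clamped Time up or down, and MoveDoor lerps both meshes in opposite directions along the actor's forward axis.
; Any overlap with the Box checks the current level name and opens Title from STAGE1, STAGE2 or STAGE3.
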(event `self.ReceiveBeginPlay`
  (bind _output_get (set `self.startposition1` (`SceneComponent.K2_GetComponentLocation` (`self.StaticMesh1`))))
  (set `self.movedposition1` (- _output_get (* (`self.GetActorForwardVector`) (`self.move`))))
  (bind _output_get_2 (set `self.startposition2` (`SceneComponent.K2_GetComponentLocation` (`self.StaticMesh2`))))
  (set `self.Movedposition2` (+ _output_get_2 (* (`self.GetActorForwardVector`) (`self.move`)))))

(event `self.ReceiveActorBeginOverlap`
  (params (OtherActor :type "Actor Object Reference"))
  (cast `/Game/FirstPersonBP/Blueprints/FirstPersonCharacter` OtherActor)
  (set `self.hit` true)
  (set `self.movevec` 1.0))

(event `self.ReceiveTick`
  (params (DeltaSeconds :type "Float (single-precision)"))
  ;[1 1 1] プレイヤーがSphereの中に入っていればドアを開ける
  ; プレイヤーがSphereの中に入っていなければドアを閉める
  (if (`self.hit`)
    (set `self.time` (`KismetMathLibrary.FClamp` (+ DeltaSeconds (`self.time`))))
    (else
      (set `self.time` (`KismetMathLibrary.FClamp` (- (`self.time`) DeltaSeconds)))))
  ;;[1 1 1] ドアの開閉
  (`self.Move Door`))

(event `self.Sphere.OnComponentEndOverlap`
  (params (OverlappedComponent :type "PrimitiveComponent Object Reference") (OtherActor :type "Actor Object Reference") (OtherComp :type "PrimitiveComponent Object Reference") (OtherBodyIndex :type Integer))
  (cast `/Game/FirstPersonBP/Blueprints/FirstPersonCharacter` OtherActor)
  (set `self.hit` false)
  (set `self.movevec` -1.0))

(event `self.Box.OnComponentBeginOverlap`
  (params (OverlappedComponent :type "PrimitiveComponent Object Reference") (OtherActor :type "Actor Object Reference") (OtherComp :type "PrimitiveComponent Object Reference") (OtherBodyIndex :type Integer) (bFromSweep :type Boolean) (SweepResult :type "HitResult Structure (by ref)"))
  ;[1 1 1] 現在のレベルによって遷移するレベルを変える
  (bind _returnvalue (`GameplayStatics.GetCurrentLevelName` true))
  (switch `string` _returnvalue
    (:`STAGE1`
      (`GameplayStatics.OpenLevelBySoftObjectPtr` "/Game/FirstPersonBP/Maps/Title.Title"))
    (:`STAGE2`
      (`GameplayStatics.OpenLevelBySoftObjectPtr` "/Game/FirstPersonBP/Maps/Title.Title"))
    (:`STAGE3`
      (`GameplayStatics.OpenLevelBySoftObjectPtr` "/Game/FirstPersonBP/Maps/Title.Title"))))

(fn `Move Door`
  ;[1 1 1] 扉の開閉
  (`SceneComponent.K2_SetWorldLocation` (`self.StaticMesh2`) (`KismetMathLibrary.VLerp` (`self.startposition2`) (`self.Movedposition2`) (`self.time`)) false false)
  (`SceneComponent.K2_SetWorldLocation` (`self.StaticMesh1`) (`KismetMathLibrary.VLerp` (`self.startposition1`) (`self.movedposition1`) (`self.time`)) false false))

(fn `UserConstructionScript`)