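; Laser enemy that sends the player back to the mesh location saved at BeginPlay when its beam hits them.
; Each Tick aligns the Niagara beam with StaticMesh and line-traces forward on Visibility.
; Non-player hits store HitPosition, whose largest per-axis distance from the mesh sets beam length on the following Tick.
; A constant-true branch leaves NoHitLength unused, so misses keep the last hit point.
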(event `self.ReceiveBeginPlay`
  (set `self.playerPosition` (`SceneComponent.K2_GetComponentLocation` (`Character.Mesh` (`GameplayStatics.GetPlayerCharacter` 0)))))

(event `self.ReceiveTick`
  (params (DeltaSeconds :type "Float (single-precision)"))
  (`SceneComponent.K2_SetWorldRotation` (`self.Niagara`) (`SceneComponent.K2_GetComponentRotation` (`self.StaticMesh`)) false false)
  (bind _newparam (`self.FindLaserLength`))
  (`NiagaraComponent.SetNiagaraVariableVec3` (`self.Niagara`) "endPosition" (`KismetMathLibrary.MakeVector` _newparam))
  ;[1 1 1] 線分の伸ばして線上にオブジェクトが当たっているか判定
  (bind (_startposition _endposition) (`self.LineStartPosition`))
  (bind (_outhit _returnvalue) (`KismetSystemLibrary.LineTraceSingle` :`Start` _startposition :`End` _endposition :`TraceChannel` "TraceTypeQuery1" :`TraceColor` (struct :`R` 1.0 :`B` 0.014804 :`A` 1.0) :`TraceHitColor` (struct :`R` 1.0) :`DrawTime` 1000.0))
  (bind _output_get (set `self.hit` _returnvalue))
  (if _output_get
    (bind (_bblockinghit _binitialoverlap _time _distance _location _impactpoint _normal _impactnormal _physmat _hitactor) (`GameplayStatics.BreakHitResult` _outhit))
    (cast `/Game/FirstPersonBP/Blueprints/FirstPersonCharacter` _hitactor
      (:`then`
        (`self.K2_SetActorLocation` (`GameplayStatics.GetPlayerPawn` 0) (`self.playerPosition`) false false)
        (`KismetSystemLibrary.PrintString` "playerHit"))
      (:`CastFailed`
        (set `self.hitPosition` _location)))))

(fn `FindLaserLength`
  (returns (NewParam :type "Float (double-precision)"))
  (locals (noHitLength :type "Float (double-precision)" :default 1000.0) (length :type "Float (double-precision)"))
  (bind (_returnvalue_x _returnvalue_y _returnvalue_z) (`KismetMathLibrary.BreakVector` (`KismetMathLibrary.Vector_GetAbs` (- (`self.hitPosition`) (`SceneComponent.K2_GetComponentLocation` (`self.StaticMesh`))))))
  (if true
    (set `local.length` (`KismetMathLibrary.FMax` _returnvalue_x _returnvalue_y _returnvalue_z))
    (else
      (set `local.length` (`local.noHitLength`))))
  (return (`local.length`)))

(fn `LineStartPosition`
  (returns (startPosition :type "Vector Structure") (endPosition :type "Vector Structure"))
  (locals (LineLength :type "Float (double-precision)" :default 100000.0))
  (bind _staticmesh (`self.StaticMesh`))
  (bind _returnvalue (`SceneComponent.K2_GetComponentLocation` _staticmesh))
  (bind _returnvalue_2 (`KismetMathLibrary.GetForwardVector` (`SceneComponent.K2_GetComponentRotation` _staticmesh)))
  (bind _returnvalue_3 (+ _returnvalue (* _returnvalue_2 (`local.LineLength`))))
  (set `self.endPosition` _returnvalue_3)
  (return (+ _returnvalue (* _returnvalue_2 50.0)) _returnvalue_3))

(fn `UserConstructionScript`)