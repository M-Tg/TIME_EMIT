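; Time-manipulable object that the player can scrub backward and forward along a preset path, with physics held off.
; At BeginPlay it bakes a fine-grained transform list by interpolating through five child-actor markers to its own position.
; ControlTime steps through that list via ControlMove and CountMoveTime, lerping between samples.
; While it is the character's ControlActor, Tick tints it by direction and spawns matching particle actors; free-physics recording is left unwired.
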(event `Count Free Time`
  (params (`Delta seconds` :type "Float (double-precision)"))
  ;[1 1 1] 単位時間に達したら差分情報を保存
  ;;[1 1 1] 自由時間計測
  (bind _output_get (set `self.NowFreeTime` (+ (`KismetMathLibrary.FClamp` `Delta seconds` 0.0 (`self.Unit Time`)) (stale _output_get))))
  (if (>= _output_get (`self.Unit Time`))
    (bind _output_get_2 (set `self.NowFreeTime` (- (stale _output_get_2) (`self.Unit Time`))))
    (`self.Set Delta` (`SceneComponent.K2_GetComponentToWorld` (`self.Object`)))))

(event `Be Free`
  (bind _object (`self.Object`))
  ;[1 1 1] 状態変化
  (`PrimitiveComponent.SetSimulatePhysics` _object true)
  (`PrimitiveComponent.SetMassOverrideInKg` _object "None" 100.0 true)
  (set `self.Free` true))

(event `Stop Time`
  (bind _object (`self.Object`))
  ;[1 1 1] 状態変化
  (`PrimitiveComponent.SetSimulatePhysics` _object false)
  (set `self.Free` false)
  (`PrimitiveComponent.SetCollisionProfileName` _object "BlockAll" true))

(event `Set Delta`
  (params (NowTransform :type "Transform Structure"))
  ;[1 1 1] 単位時間に達したら差分情報を保存
  ;;[1 1 1] 差分保存
  (`KismetArrayLibrary.Array_Add` (`self.TransformList`) NowTransform)
  (set `self.NowTransform` (`SceneComponent.K2_GetComponentToWorld` (`self.Object`))))

(event `self.ReceiveBeginPlay`
  (`self.EffectFirstSet`)
  (`self.Stop Time`)
  (`self.CreateTransformList`))

(event `self.ReceiveTick`
  (params (DeltaSeconds :type "Float (single-precision)"))
  (`self.Stop Time`)
  ;[1 1 1] 時間移動指定されているか
  (if (== (`/Game/FirstPersonBP/Blueprints/FirstPersonCharacter.Control Actor` (cast `/Game/FirstPersonBP/Blueprints/FirstPersonCharacter` (`GameplayStatics.GetPlayerCharacter` 0) :!pure true)) self)
    ;[1 1 1] エフェクトを追加
    (switch `/Game/Contents/BP_Enum_Object_State` (`self.State`)
      (:`NewEnumerator0`
        (`self.SetEffectMatrial` (struct :`B` 1.0 :`A` 1.0) :!label _label))
      (:`NewEnumerator2`
        (goto _label))
      (:`NewEnumerator3`
        (`self.SetEffectMatrial` (struct :`R` 1.0 :`A` 1.0) true)))
    (else
      ;[1 1 1] マテリアルを元に戻す
      (`self.BackToBase`))))

(event `Count Move Time`
  (params (`Move Seconds` :type "Float (double-precision)"))
  ;[1 1 1] 自由時間停止中の移動操作
  ;;[1 1 1] 移動時間カウント
  (if (>= `Move Seconds` 0.0)
    ;;;[1 1 1] 逆移動
    (bind _output_get (set `self.MoveTime` (+ `Move Seconds` (stale _output_get))))
    (`self.Time Transform` 0.0 (- (- (`self.MaxSection`) 1) (`self.NowSection`)))
    (if (>= (`self.MoveTime`) (`self.Unit Time`))
      (`/Engine/EditorBlueprintResources/StandardMacros.IncrementInt` (`self.NowSection`)
        (:`  `
          (set `self.MoveTime` 0.0 :!label _label_2)
          (set `self.NowTransform` (`SceneComponent.K2_GetComponentToWorld` (`self.Object`))))))
    (else
      ;;[1 1 1] 正移動
      (bind _output_get_2 (set `self.MoveTime` (+ (* `Move Seconds` -1.0) (stale _output_get_2))))
      (`self.Time Transform` 0.0 (- (`self.MaxSection`) (`self.NowSection`)))
      (if (>= (`self.MoveTime`) (`self.Unit Time`))
        (`/Engine/EditorBlueprintResources/StandardMacros.DecrementInt` (`self.NowSection`)
          (:`  `
            (goto _label_2)))))))

(event `Time Transform`
  (params (`Move Seconds` :type "Float (double-precision)") (Index :type Integer))
  ;[1 1 1] 自由時間停止中の移動操作
  ;;[1 1 1] 差分移動
  (`SceneComponent.K2_SetWorldTransform` (`self.Object`) (`KismetMathLibrary.TLerp` (`self.NowTransform`) (`|GetArrayItem` (`self.TransformList`) Index) (/ (`self.MoveTime`) (`self.Unit Time`))) false false))

(event `SetEffectMatrial`
  (params (Value :type "LinearColor Structure") (Invert :type Boolean))
  ;[1 1 1] エフェクト材質を与える＋色付け
  (bind _returnvalue (`PrimitiveComponent.CreateDynamicMaterialInstance` (`self.Object`) 0 (`self.EffectMaterial`) "None"))
  (`MaterialInstanceDynamic.SetVectorParameterValue` _returnvalue "Color" Value)
  (`self.CreateEffect` Value Invert))

(event `BackToBase`
  ;[1 1 1] 元のMaterialに戻る
  (`PrimitiveComponent.CreateDynamicMaterialInstance` (`self.Object`) 0 (`self.baseMaterial`) "None"))

(event `EffectFirstSet`
  (bind _object (`self.Object`))
  ;[1 1 1] 最初に呼び出す
  ;;[1 1 1] 元のエフェクトを得る
  (set `self.baseMaterial` (`PrimitiveComponent.GetMaterial` _object 0))
  (bind _returnvalue (`PrimitiveComponent.CreateDynamicMaterialInstance` _object 0 "/Game/Contents/Materials/M_TimeMoving_Inst.M_TimeMoving_Inst" "None"))
  (set `self.EffectMaterial` _returnvalue)
  (`self.BackToBase`))

(fn `Control Move`
  (params (`Move Seconds` :type "Float (double-precision)"))
  (returns (moved :type Boolean))
  (bind _unit_time (`self.Unit Time`))
  (if (>= `Move Seconds` 0.0)
    ;[1 1 1] 進行方向の最終タイミングでないか
    (if (> (`self.MaxSection`) (`self.NowSection`))
      _
      (else
        (set `self.State` "NewEnumerator1" :!label _label)
        ;[1 1 1] 動けたかを返す
        (return false)))
    (elif (> (`self.NowSection`) 0)
      _
      (else
        (goto _label))))
  (`self.Count Move Time` (`KismetMathLibrary.FClamp` `Move Seconds` (* _unit_time -1.0) _unit_time))
  (return true))

(fn `Control Time`
  (params (Invert :type Boolean))
  (returns (`Can Move` :type Boolean))
  (bind _min_move_sec (`self.MIn Move Sec`))
  (if (not (`self.Free`))
    (if Invert
      ;[1 1 1] 逆行
      (bind _moved (`self.Control Move` _min_move_sec))
      (set `self.State` "NewEnumerator3")
      (return _moved)
      (else
        ;[1 1 1] 順行
        (bind _moved_2 (`self.Control Move` (* _min_move_sec -1.0)))
        (set `self.State` "NewEnumerator2")
        (return _moved_2)))
    (else
      (return false))))

(fn `CreateEffect`
  (params (EffectColor :type "LinearColor Structure") (Invert :type Boolean))
  (bind _returnvalue (* (0.2 0.2 0.2) 1.0))
  (bind _effectbox (`self.EffectBox`))
  (bind _returnvalue_2 (`SceneComponent.K2_GetComponentLocation` _effectbox))
  (bind _returnvalue_3 (`KismetMathLibrary.MakeTransform` _returnvalue_2 (struct) _returnvalue))
  (bind _returnvalue_4 (+ _returnvalue_2 (`KismetMathLibrary.GreaterGreater_VectorRotator` (* (`BoxComponent.GetScaledBoxExtent` _effectbox) (`KismetMathLibrary.MakeVector` (`KismetMathLibrary.RandomFloatInRange` -1.0 1.0) (`KismetMathLibrary.RandomFloatInRange` -1.0 1.0) (`KismetMathLibrary.RandomFloatInRange` -1.0 1.0)) (1.0 1.0 1.0)) (`SceneComponent.K2_GetComponentRotation` _effectbox))))
  (bind _returnvalue_5 (`KismetMathLibrary.MakeTransform` _returnvalue_4 (struct) (* _returnvalue 1.0)))
  (if Invert
    (`|SpawnActorFromClass` "/Game/Contents/Effect/Ef_Base_Recive.Ef_Base_Recive_C" _returnvalue_3 "Undefined" "OverrideRootScale" null EffectColor _returnvalue_4 null)
    (`|SpawnActorFromClass` "/Game/Contents/Effect/Ef_Base_ReciveSide.Ef_Base_ReciveSide_C" _returnvalue_5 "Undefined" "OverrideRootScale" null (struct :`R` 1.0 :`G` 0.406108 :`A` 1.0) null)
    (else
      (`|SpawnActorFromClass` "/Game/Contents/Effect/Ef_Base_Give.Ef_Base_Give_C" _returnvalue_3 "Undefined" "OverrideRootScale" null EffectColor _returnvalue_4 null)
      (`|SpawnActorFromClass` "/Game/Contents/Effect/Ef_Base_GiveSide.Ef_Base_GiveSide_C" _returnvalue_5 "Undefined" "OverrideRootScale" null (struct :`G` 0.925398 :`B` 1.0 :`A` 1.0) null))))

(fn `CreateTransformList`
  (locals (`total time` :type "Float (double-precision)") (`now section` :type Integer :default 0))
  (bind _seconds_transform_list (`self.seconds transform list`))
  (bind _seconds_transform_list_2 (`self.seconds transform list`))
  (bind _returnvalue (`KismetMathLibrary.FTrunc` (`local.total time`)))
  (bind _returnvalue_2 (`KismetMathLibrary.FTrunc` (`local.total time`)))
  (bind _returnvalue_3 (`SceneComponent.K2_GetComponentToWorld` (`self.Object`)))
  ;[1 1 1] 子アクタの場所を1秒ごとに設定する
  (`KismetArrayLibrary.Array_Add` _seconds_transform_list (`SceneComponent.K2_GetComponentToWorld` (`self.ChildActor1`)))
  (`KismetArrayLibrary.Array_Add` _seconds_transform_list (`SceneComponent.K2_GetComponentToWorld` (`self.ChildActor2`)))
  (`KismetArrayLibrary.Array_Add` _seconds_transform_list (`SceneComponent.K2_GetComponentToWorld` (`self.ChildActor3`)))
  (`KismetArrayLibrary.Array_Add` _seconds_transform_list (`SceneComponent.K2_GetComponentToWorld` (`self.ChildActor4`)))
  (`KismetArrayLibrary.Array_Add` _seconds_transform_list (`SceneComponent.K2_GetComponentToWorld` (`self.ChildActor5`)))
  ;[1 1 1] 最後の位置を現在位置に
  (`KismetArrayLibrary.Array_Add` _seconds_transform_list _returnvalue_3)
  (set `self.NowTransform` _returnvalue_3)
  ;[1 1 1] 単位時間を設定
  (bind _output_get (set `self.Unit Time` 0.03))
  ;[1 1 1] Ｘ秒で何個保存されるかを設定
  (bind _output_get_2 (set `self.MaxSection` 5))
  (set `self.MaxSection` (`KismetMathLibrary.FTrunc` (* _output_get_2 (/ 1.0 _output_get))))
  ;[1 1 1] 移動経過用時間を設定
  (set `self.MIn Move Sec` (/ (`self.Unit Time`) 1.0))
  ;[1 1 1] 指定秒数分の保存をする
  (while (< (`KismetArrayLibrary.Array_Length` (`self.TransformList`)) (`self.MaxSection`))
    ;[1 1 1] １秒までの変化を単位時間ごとに保存
    (`self.Set Delta` (`|EaseFunction` "Linear" (- (`local.total time`) (`KismetMathLibrary.Conv_IntToDouble` (`local.now section`))) (`|GetArrayItem` _seconds_transform_list_2 _returnvalue) (`|GetArrayItem` _seconds_transform_list_2 (+ _returnvalue 1))))
    ;;[1 1 1] 時間計測
    (bind _output_get_3 (set `local.total time` (+ (stale _output_get_3) (`self.Unit Time`))))
    (if (!= (stale _output_get_4) _returnvalue_2)
      (bind _output_get_4 (set `local.now section` _returnvalue_2)))))

(fn `UserConstructionScript`
  (`ChildActorComponent.SetChildActorClass` (`self.ChildActor1`) "/Game/Contents/BP_MovedPosition.BP_MovedPosition_C")
  (`ChildActorComponent.SetChildActorClass` (`self.ChildActor2`) "/Game/Contents/BP_MovedPosition.BP_MovedPosition_C")
  (`ChildActorComponent.SetChildActorClass` (`self.ChildActor3`) "/Game/Contents/BP_MovedPosition.BP_MovedPosition_C")
  (`ChildActorComponent.SetChildActorClass` (`self.ChildActor4`) "/Game/Contents/BP_MovedPosition.BP_MovedPosition_C")
  (`ChildActorComponent.SetChildActorClass` (`self.ChildActor5`) "/Game/Contents/BP_MovedPosition.BP_MovedPosition_C"))