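; BP_MoveObjectBase_M is a movable-object Blueprint that precomputes a six-second path of transforms for its Object, starting at the midpoint.
; Its CreateTransformList override, which skips the parent version, takes seven one-second keyframes: three child actors, the Object, then three more.
; It linearly interpolates these at a fixed small time step via SetDelta to build TransformList.
; The construction script sets ChildActor6 to BP_MovedPosition; event graph nodes are disabled placeholders.
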(fn `CreateTransformList`
  (locals (`total time` :type "Float (double-precision)") (`now second section` :type Integer))
  (bind _seconds_transform_list (`self.seconds transform list`))
  (bind _seconds_transform_list_2 (`self.seconds transform list`))
  (bind _returnvalue (`KismetMathLibrary.FTrunc` (`local.total time`)))
  (bind _returnvalue_2 (`KismetMathLibrary.FTrunc` (`local.total time`)))
  (bind _returnvalue_3 (`SceneComponent.K2_GetComponentToWorld` (`self.Object`)))
  ;[1 1 1] 子アクタの場所を1秒ごとに設定する
  (`KismetArrayLibrary.Array_Add` _seconds_transform_list (`SceneComponent.K2_GetComponentToWorld` (`self.ChildActor1`)))
  (`KismetArrayLibrary.Array_Add` _seconds_transform_list (`SceneComponent.K2_GetComponentToWorld` (`self.ChildActor2`)))
  (`KismetArrayLibrary.Array_Add` _seconds_transform_list (`SceneComponent.K2_GetComponentToWorld` (`self.ChildActor3`)))
  ;[1 1 1] 真ん中の位置を現在位置に
  (`KismetArrayLibrary.Array_Add` _seconds_transform_list _returnvalue_3)
  (set `self.NowTransform` _returnvalue_3)
  (`KismetArrayLibrary.Array_Add` _seconds_transform_list (`SceneComponent.K2_GetComponentToWorld` (`self.ChildActor4`)))
  (`KismetArrayLibrary.Array_Add` _seconds_transform_list (`SceneComponent.K2_GetComponentToWorld` (`self.ChildActor5`)))
  (`KismetArrayLibrary.Array_Add` _seconds_transform_list (`SceneComponent.K2_GetComponentToWorld` (`self.ChildActor6`)))
  ;[1 1 1] 単位時間を設定
  (bind _output_get (set `self.Unit Time` 0.03))
  ;[1 1 1] Ｘ秒で何個保存されるかを設定
  (bind _output_get_2 (set `self.MaxSection` 6))
  (bind _returnvalue_4 (/ 1.0 _output_get))
  (set `self.MaxSection` (`KismetMathLibrary.FTrunc` (* _output_get_2 _returnvalue_4)))
  (set `self.NowSection` (`KismetMathLibrary.FTrunc` (* 3 _returnvalue_4)))
  ;[1 1 1] 移動経過用時間を設定
  (set `self.MIn Move Sec` (/ (`self.Unit Time`) 1.0))
  ;[1 1 1] 指定秒数分の保存をする
  (while (< (`KismetArrayLibrary.Array_Length` (`self.TransformList`)) (`self.MaxSection`))
    ;[1 1 1] １秒までの変化を単位時間ごとに保存
    (`self.Set Delta` (`|EaseFunction` "Linear" (- (`local.total time`) (`KismetMathLibrary.Conv_IntToDouble` (`local.now second section`))) (`|GetArrayItem` _seconds_transform_list_2 _returnvalue) (`|GetArrayItem` _seconds_transform_list_2 (+ _returnvalue 1))))
    ;;[1 1 1] 時間計測
    (bind _output_get_3 (set `local.total time` (+ (stale _output_get_3) (`self.Unit Time`))))
    (if (!= (stale _output_get_4) _returnvalue_2)
      (bind _output_get_4 (set `local.now second section` _returnvalue_2)))))

(fn `UserConstructionScript`
  (`parent.UserConstructionScript`)
  (`ChildActorComponent.SetChildActorClass` (`self.ChildActor6`) "/Game/Contents/BP_MovedPosition.BP_MovedPosition_C"))