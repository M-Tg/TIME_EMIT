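; Base actor for a time-manipulable object that simulates physics briefly, then freezes so its recorded motion can be scrubbed.
; Tick samples world transforms at fixed intervals until the list is full, then disables physics.
; ControlTime steps backward or forward through the recording via ControlMove, lerping between stored transforms.
; While it is the FirstPersonCharacter's ControlActor, direction-colored materials and effect actors spawned around EffectBox show the time flow.
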(event `Count Free Time`
  (params (`Delta seconds` :type "Float (double-precision)"))
  ;[1 1 1] 単位時間に達したら差分情報を保存
  ;;[1 1 1] 自由時間計測
  (bind _output_get (set `self.NowFreeTime` (+ (`KismetMathLibrary.FClamp` `Delta seconds` 0.0 (`self.Unit Time`)) (stale _output_get))))
  (if (>= _output_get (`self.Unit Time`))
    (bind _output_get_2 (set `self.NowFreeTime` (- (stale _output_get_2) (`self.Unit Time`))))
    (`self.Set Delta`)))

(event `Be Free`
  (bind _object (`self.Object`))
  ;[1 1 1] 状態変化
  (`PrimitiveComponent.SetSimulatePhysics` _object true)
  (`PrimitiveComponent.SetMassOverrideInKg` _object "None" 100.0 true)
  (set `self.Free` true)
  (`MaterialInstanceDynamic.SetVectorParameterValue` (`self.Material`) "Color" (struct :`R` 0.777181 :`G` 0.78125 :`B` 0.773112 :`A` 1.0)))

(event `Stop Time`
  (bind _object (`self.Object`))
  ;[1 1 1] 状態変化
  (`PrimitiveComponent.SetSimulatePhysics` _object false)
  (set `self.Free` false)
  (`PrimitiveComponent.SetCollisionProfileName` _object "BlockAll" true)
  (`MaterialInstanceDynamic.SetVectorParameterValue` (`self.Material`) "Color" (struct :`R` 0.067708 :`G` 0.0614 :`B` 0.064193 :`A` 1.0)))

(event `Set Delta`
  ;[1 1 1] 単位時間に達したら差分情報を保存
  ;;[1 1 1] 差分保存
  (`KismetArrayLibrary.Array_Add` (`self.TransformList`) (`SceneComponent.K2_GetComponentToWorld` (`self.Object`)))
  (set `self.NowTransform` (`SceneComponent.K2_GetComponentToWorld` (`self.Object`))))

(event `self.ReceiveBeginPlay`
  (`self.EffectFirstSet`)
  (`self.Be Free`)
  (set `self.NowTransform` (`SceneComponent.K2_GetComponentToWorld` (`self.Object`)))
  ;[1 1 1] 単位時間を設定
  (bind _output_get (set `self.Unit Time` 0.03))
  ;[1 1 1] Ｘ秒で何個保存されるかを設定
  (bind _output_get_2 (set `self.MaxSection` 5))
  (set `self.MaxSection` (`KismetMathLibrary.FTrunc` (* _output_get_2 (/ 1.0 _output_get))))
  ;[1 1 1] 移動経過用時間を設定
  (set `self.MIn Move Sec` (/ (`self.Unit Time`) 1.0)))

(event `self.ReceiveTick`
  (params (DeltaSeconds :type "Float (single-precision)"))
  (if (< (`KismetArrayLibrary.Array_Length` (`self.TransformList`)) (`self.MaxSection`))
    (`self.Count Free Time` DeltaSeconds)
    (else
      (`self.Stop Time`)
      (if (== (`/Game/FirstPersonBP/Blueprints/FirstPersonCharacter.Control Actor` (cast `/Game/FirstPersonBP/Blueprints/FirstPersonCharacter` (`GameplayStatics.GetPlayerCharacter` 0) :!pure true)) self)
        (`MaterialInstanceDynamic.SetVectorParameterValue` (`self.Material`) "Color" (struct :`R` 0.510417 :`B` 0.459142 :`A` 1.0))
        (switch `/Game/Contents/BP_Enum_Object_State` (`self.State`)
          (:`NewEnumerator2`
            (`self.SetEffectMatrial` (struct :`B` 1.0 :`A` 1.0)))
          (:`NewEnumerator3`
            (`self.SetEffectMatrial` (struct :`R` 1.0 :`A` 1.0) true)))
        (else
          (`self.BackToBase`))))))

(event `Time Transform`
  (params (`Move Seconds` :type "Float (double-precision)") (Index :type Integer))
  ;[1 1 1] 自由時間停止中の移動操作
  ;;[1 1 1] 差分移動
  (`SceneComponent.K2_SetWorldTransform` (`self.Object`) (`KismetMathLibrary.TLerp` (`self.NowTransform`) (`|GetArrayItem` (`self.TransformList`) Index) (/ (`self.MoveTime`) (`self.Unit Time`))) false false))

(event `Count Move Time`
  (params (`Move Seconds` :type "Float (double-precision)"))
  ;[1 1 1] 自由時間停止中の移動操作
  ;;[1 1 1] 移動時間カウント
  (if (>= `Move Seconds` 0.0)
    (bind _output_get (set `self.MoveTime` (+ `Move Seconds` (stale _output_get))))
    (`self.Time Transform` 0.0 (- (- (`self.MaxSection`) 1) (`self.NowSection`)))
    (if (>= (`self.MoveTime`) (`self.Unit Time`))
      (`/Engine/EditorBlueprintResources/StandardMacros.IncrementInt` (`self.NowSection`)
        (:`  `
          (set `self.MoveTime` 0.0 :!label _label)
          (set `self.NowTransform` (`SceneComponent.K2_GetComponentToWorld` (`self.Object`))))))
    (else
      (bind _output_get_2 (set `self.MoveTime` (+ (* `Move Seconds` -1.0) (stale _output_get_2))))
      (`self.Time Transform` 0.0 (- (`self.MaxSection`) (`self.NowSection`)))
      (if (>= (`self.MoveTime`) (`self.Unit Time`))
        (`/Engine/EditorBlueprintResources/StandardMacros.DecrementInt` (`self.NowSection`)
          (:`  `
            (goto _label)))))))

(event `SetEffectMatrial`
  (params (Value :type "LinearColor Structure") (Invert :type Boolean))
  ;[1 1 1] エフェクト材質を与える＋色付け
  (bind _returnvalue (`PrimitiveComponent.CreateDynamicMaterialInstance` (`self.Object`) 0 (`self.EffectMaterial`) "None"))
  (`MaterialInstanceDynamic.SetVectorParameterValue` _returnvalue "Color" Value)
  (`self.CreateEffect` Value Invert))

(event `EffectFirstSet`
  (bind _object (`self.Object`))
  ;[1 1 1] 最初に呼び出す
  ;;[1 1 1] 元のエフェクトを得る
  (set `self.baseMaterial` (`PrimitiveComponent.GetMaterial` _object 0))
  (bind _returnvalue (`PrimitiveComponent.CreateDynamicMaterialInstance` _object 0 "/Game/Contents/Materials/M_TimeMoving_Inst.M_TimeMoving_Inst" "None"))
  (set `self.EffectMaterial` _returnvalue)
  (`self.BackToBase`))

(event `BackToBase`
  ;[1 1 1] 元のMaterialに戻る
  (`PrimitiveComponent.CreateDynamicMaterialInstance` (`self.Object`) 0 (`self.baseMaterial`) "None"))

(fn `Control Move`
  (params (`Move Seconds` :type "Float (double-precision)"))
  (returns (moved :type Boolean))
  (bind _unit_time (`self.Unit Time`))
  (if (>= `Move Seconds` 0.0)
    ;[1 1 1] 進行方向の最終タイミングでないか
    (if (> (`self.MaxSection`) (`self.NowSection`))
      _
      (else
        (set `self.State` "NewEnumerator1" :!label _label)
        ;[1 1 1] 動けたかを返す
        (return false)))
    (elif (> (`self.NowSection`) 0)
      _
      (else
        (goto _label))))
  (`self.Count Move Time` (`KismetMathLibrary.FClamp` `Move Seconds` (* _unit_time -1.0) _unit_time))
  (return true))

(fn `Control Time`
  (params (Invert :type Boolean))
  (returns (`Can Move` :type Boolean))
  (bind _min_move_sec (`self.MIn Move Sec`))
  (bind _material (`self.Material`))
  (if (not (`self.Free`))
    (if Invert
      ;[1 1 1] 逆行
      (bind _moved (`self.Control Move` _min_move_sec))
      (`MaterialInstanceDynamic.SetVectorParameterValue` _material "Color" (struct :`R` 1.0 :`G` 0.01768 :`A` 1.0))
      (set `self.State` "NewEnumerator3")
      (return _moved)
      (else
        ;[1 1 1] 順行
        (bind _moved_2 (`self.Control Move` (* _min_move_sec -1.0)))
        (`MaterialInstanceDynamic.SetVectorParameterValue` _material "Color" (struct :`R` 0.173035 :`B` 1.0 :`A` 1.0))
        (set `self.State` "NewEnumerator2")
        (return _moved_2)))
    (else
      (return false))))

(fn `CreateEffect`
  (params (EffectColor :type "LinearColor Structure") (Invert :type Boolean))
  (bind _returnvalue (* (0.2 0.2 0.2) 1.0))
  (bind _effectbox (`self.EffectBox`))
  (bind _returnvalue_2 (`SceneComponent.K2_GetComponentLocation` _effectbox))
  (bind _returnvalue_3 (`BoxComponent.GetScaledBoxExtent` _effectbox))
  (bind _returnvalue_4 (`KismetMathLibrary.MakeTransform` _returnvalue_2 (struct) _returnvalue))
  (bind _returnvalue_5 (+ (- _returnvalue_2 (/ _returnvalue_3 1.0)) (* _returnvalue_3 (`KismetMathLibrary.MakeVector` (`KismetMathLibrary.RandomFloatInRange` 0.0 1.0) (`KismetMathLibrary.RandomFloatInRange` 0.0 1.0) (`KismetMathLibrary.RandomFloatInRange` 0.0 1.0)) (2.0 2.0 2.0))))
  (bind _returnvalue_6 (`KismetMathLibrary.MakeTransform` (+ _returnvalue_5 (0.0 0.0 0.0)) (struct) (* _returnvalue 1.0)))
  (if Invert
    (`|SpawnActorFromClass` "/Game/Contents/Effect/Ef_Base_Recive.Ef_Base_Recive_C" _returnvalue_4 "Undefined" "OverrideRootScale" null EffectColor _returnvalue_5 null)
    (for _ (range 9)
      (`|SpawnActorFromClass` "/Game/Contents/Effect/Ef_Base_ReciveSide.Ef_Base_ReciveSide_C" _returnvalue_6 "Undefined" "OverrideRootScale" null (struct :`R` 1.0 :`G` 0.406108 :`A` 1.0) null))
    (else
      (`|SpawnActorFromClass` "/Game/Contents/Effect/Ef_Base_Give.Ef_Base_Give_C" _returnvalue_4 "Undefined" "OverrideRootScale" null EffectColor _returnvalue_5 null)
      (for _ (range 9)
        (`|SpawnActorFromClass` "/Game/Contents/Effect/Ef_Base_GiveSide.Ef_Base_GiveSide_C" _returnvalue_6 "Undefined" "OverrideRootScale" null (struct :`G` 0.925398 :`B` 1.0 :`A` 1.0) null)))))

(fn `UserConstructionScript`
  (bind _returnvalue (`KismetMaterialLibrary.CreateDynamicMaterialInstance` "/Game/Contents/M_Test.M_Test" "Color"))
  (bind _output_get (set `self.Material` _returnvalue))
  (`PrimitiveComponent.SetMaterial` (`self.Object`) 0 _output_get))